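; MagicStone is an interactable world object, a glowing stone that can be taken.
; Its construction script sets the display name and description and builds an interaction structure with two interaction types, pointing to itself.
; The Take event passes the interactor to OnTake, and only on success calls Save and destroys the actor.
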(event EventTake
  (params (Interactor :type Actor%20Object%20Reference))
  (bind _success (CallFunction|OnTake Interactor))
  (if _success
    (CallFunction|Save)
    (Actor|DestroyActor)))

(fn ConstructionScript
  (Variables|Default|SetName "Stone")
  (Variables|Default|SetInfo "Mystically glowing stone that pulses with strange energy.")
  (Variables|Default|SetInteractions (Utilities|Struct|MakeInteractionStructure (Utilities|Array|MakeArray "NewEnumerator0" "NewEnumerator3") self)))