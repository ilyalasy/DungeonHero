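; Interactable object that shows its name on the HUD and accepts Interact input when the player character faces it.
; Every Tick it line-traces from the character along its forward vector: hitting this actor enables input, while hitting nothing clears the name and disables input.
; Hitting a different actor changes neither.
; Interact passes the Interactions variable to MyHUD, cached at BeginPlay; the Open event is an empty stub.
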(event EventOpen)

(event EventTick
  (params (DeltaSeconds :type Float%20%28single-precision%29))
  (bind _returnvalue (Game|GetPlayerCharacter 0))
  (bind _returnvalue_2 (Transformation|GetActorLocation _returnvalue))
  ;[1 1 1] Determine whether character looking at this object or not
  (bind (_outhit _returnvalue_3) (Collision|LineTraceByChannel _returnvalue_2 (+ _returnvalue_2 (* (Transformation|GetActorForwardVector _returnvalue) (Variables|Default|GetTraceDistance))) "TraceTypeQuery1" false 0 "None" false))
  (if _returnvalue_3
    (if (== (.HitActor (Collision|BreakHitResult _outhit)) self)
      (Default|CallUpdateActorNameWidget (stale EventBeginPlay _output_get) (Variables|Default|GetName))
      (Input|EnableInput (stale EventBeginPlay _output_get_2)))
    (else
      (Default|CallUpdateActorNameWidget (stale EventBeginPlay _output_get) " ")
      (Input|DisableInput (stale EventBeginPlay _output_get_2)))))

(event EventBeginPlay
  (bind _returnvalue (Game|GetPlayerController 0))
  ;[1 1 1] Initialize variables
  (bind _asmy_hud (Utilities|Casting|CastToMyHUD (HUD|GetHUD _returnvalue)))
  (bind _output_get (Variables|Default|SetMyHUDRef _asmy_hud))
  (bind _output_get_2 (Variables|Default|SetPlayerController _returnvalue)))

(event Input|ActionEvents|InputActionInteract
  (params (Key :type Key%20Structure :default "None"))
  (:Pressed
    (Default|CallInteractwithObject (stale EventBeginPlay _output_get) (Variables|Default|GetInteractions))))

(fn ConstructionScript)