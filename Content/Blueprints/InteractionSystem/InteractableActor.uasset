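; InteractableActor is a world object that players can inspect and interact with through the player's HUD.
; Its events show or hide the object's name, open an interaction menu with its Interactions and the interactor, and open an examine window with its Name and Info.
; Every event routes through a GetHUD helper that casts the first player controller's HUD to MyHUD.
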(event EventShowName
  (bind _asmy_hud (Utilities|GetHUD))
  (Default|ShowObjectName _asmy_hud (Variables|Default|GetName)))

(event EventHideName
  (bind _asmy_hud (Utilities|GetHUD))
  (Default|HideObjectName _asmy_hud))

(event EventInteract
  (params (Interactor :type Actor%20Object%20Reference))
  (bind _asmy_hud (Utilities|GetHUD))
  (Default|OpenInteractMenu _asmy_hud (Variables|Default|GetInteractions) Interactor))

(event EventExamine
  (bind _asmy_hud (Utilities|GetHUD))
  (Default|CreateExamineWindow _asmy_hud (Variables|Default|GetName) (Variables|Default|GetInfo)))

(fn ConstructionScript)