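; Player character that handles movement, look input, camera-trace interaction with Interactable objects, save/load of its transform, and fade-out sleep and game over.
; Inventory events attach a torch or knife to hand sockets, or loop a magic stone sound.
; Forward input triggers distance-based footsteps, using a downward trace and FlipFlops to alternate sounds per surface.
; Helper functions filter NPC dialogue answers by inventory and quest state.
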(event OnInventoryRemove(InventoryComponent)
  (params (RemovedItem :type Slot%20Structure%20Structure))
  (bind _stoneaudio (Variables|Default|GetStoneAudio))
  (Utilities|Casting|CastToTorchClass (.item (.item RemovedItem))
    (:then
      (Actor|DestroyActor (Variables|Default|GetTorch)))
    (:CastFailed
      (Utilities|Casting|CastToMagicStoneClass (.item (.item RemovedItem))
        (:then
          (Audio|Components|Audio|Stop _stoneaudio)
          (Components|DestroyComponent _stoneaudio))
        (:CastFailed
          (Utilities|Casting|CastToKnifeClass (.item (.item RemovedItem)))
          (Actor|DestroyActor (Variables|Default|GetKnife)))))))

(event OnInventoryAdd(InventoryComponent)
  (params (AddedItem :type Slot%20Structure%20Structure))
  (bind _astorch (Utilities|Casting|CastToTorchClass (.item (.item AddedItem)))
    (:then
      (bind _returnvalue (Game|SpawnActorfromClass :Class _astorch :SpawnTransform (Math|Transform|MakeTransform "0, 0, 0") :CollisionHandlingOverride "Undefined" :Instigator 0))
      (bind _output_get (Variables|Default|SetTorch _returnvalue))
      (Collision|SetCollisionEnabled (Variables|/Game/Blueprints/Objects/Torch/Torch.Torch_C|GetTorch _output_get) "NoCollision")
      (Transformation|AttachComponentToComponent _output_get (Variables|Default|GetRightHandSocket) "None" "KeepRelative" "KeepRelative" "KeepRelative" true))
    (:CastFailed
      (Utilities|Casting|CastToMagicStoneClass (.item (.item AddedItem))
        (:then
          (bind _returnvalue_2 (Audio|CreateSound2D "/Game/Audio/SFX/StoneWhisper/Stone_Loop_Cue.Stone_Loop_Cue" 1.0 1.0 0.0 0 true false))
          (bind _output_get_2 (Variables|Default|SetStoneAudio _returnvalue_2))
          (Audio|Components|Audio|Play _output_get_2 0.0))
        (:CastFailed
          (bind _asknife (Utilities|Casting|CastToKnifeClass (.item (.item AddedItem))))
          (bind _returnvalue_3 (Game|SpawnActorfromClass :Class _asknife :SpawnTransform (Math|Transform|MakeTransform "0, 0, 0" "-90.000000, 0,20.000000") :CollisionHandlingOverride "Undefined" :Instigator 0))
          (bind _output_get_3 (Variables|Default|SetKnife _returnvalue_3))
          (Collision|SetCollisionEnabled (Variables|/Game/Blueprints/Objects/Knife.Knife_C|GetKnifeMesh _output_get_3) "NoCollision")
          (Transformation|AttachComponentToComponent _output_get_3 (Variables|Default|GetLeftHandSocket) "None" "KeepRelative" "KeepRelative" "KeepRelative" true))))))

(event Custom|Step
  (Utilities|PlaySoundonMaterial))

(event Custom|Sleep
  (CameraFades|StartCameraFade :self (Game|GetPlayerCameraManager 0) :ToAlpha 1.0 :Duration 2.0 :bShouldFadeAudio true :bHoldWhenFinished true)
  (Utilities|FlowControl|Delay 2.0)
  (bind _returnvalue (Game|GetCurrentLevelName true))
  (Game|OpenLevel(byName) (Utilities|String|StringToName _returnvalue)))

(event Custom|SetSpeed_Event
  (params (NewSpeed :type Float%20%28single-precision%29))
  (Variables|/Script/Engine.CharacterMovementComponent|SetMaxWalkSpeed (Variables|Character|GetCharacterMovement) NewSpeed))

(event EventBeginPlay
  (bind _returnvalue (Game|GetPlayerController 0))
  ;[1 1 1] Enable input and get HUD ref
  (Input|EnableInput _returnvalue)
  (bind _asmy_hud (Utilities|Casting|CastToMyHUD (HUD|GetHUD _returnvalue)))
  (Variables|Default|SetHUDRef _asmy_hud)
  (CallFunction|Load))

(event EventSave
  (bind _savegame (CallFunction|GetWorldSave))
  (Utilities|Map|Add (Variables|/Game/Blueprints/Save/WorldSaveGame.WorldSaveGame_C|GetActorsTransforms _savegame) (Utilities|GetObjectName self) (Transformation|GetActorTransform))
  (SaveGame|SaveGametoSlot _savegame (Variables|/Game/Blueprints/Save/WorldSaveGame.WorldSaveGame_C|GetSaveGameSlot _savegame) (Variables|/Game/Blueprints/Save/WorldSaveGame.WorldSaveGame_C|GetPlayerID _savegame))
  (Default|Save (Variables|Default|GetInventoryComponent)))

(event EventTick
  (params (DeltaSeconds :type Float%20%28single-precision%29))
  (bind (_start _end) (Utilities|GetCameraTrace))
  ;[1 1 1] Get object character looking at
  (bind (_outhit _returnvalue) (Collision|LineTraceByChannel _start _end "TraceTypeQuery1" false 0 "None"))
  ;[1 1 1] If interactable object show its name
  (if _returnvalue
    (bind _asinteractable (Utilities|Casting|CastToInteractable (.HitActor (Collision|BreakHitResult _outhit))))
    (bind _output_get (Variables|Default|SetObjectLookingAt _asinteractable))
    (Default|ShowName _output_get)
    (else
      ;[1 1 1] If not interactable or no object at all hide name of previous object
      (Utilities|IsValid (Utilities|ToObject(Interface) (Variables|Default|GetObjectLookingAt))
        (:Is%20Valid
          (Default|HideName (Variables|Default|GetObjectLookingAt))
          (Variables|Default|SetObjectLookingAt 0))))))

(event EventLoad
  (bind _savegame (CallFunction|GetWorldSave))
  (if (.ReturnValue (Utilities|Map|Find (Variables|/Game/Blueprints/Save/WorldSaveGame.WorldSaveGame_C|GetActorsTransforms _savegame) (Utilities|GetObjectName self)))
    (Pawn|SetControlRotation (Game|GetPlayerController 0) (Math|Transform|TransformRotation (.Value (Utilities|Map|Find (Variables|/Game/Blueprints/Save/WorldSaveGame.WorldSaveGame_C|GetActorsTransforms _savegame) (Utilities|GetObjectName self))) "0, 0, 0"))
    (Transformation|SetActorTransform (.Value (Utilities|Map|Find (Variables|/Game/Blueprints/Save/WorldSaveGame.WorldSaveGame_C|GetActorsTransforms _savegame) (Utilities|GetObjectName self))))))

(event Input|ActionEvents|InputActionInteract
  (params (Key :type Key%20Structure :default "None"))
  (bind _objectlookingat (Variables|Default|GetObjectLookingAt))
  ;[1 1 1] Interact with object currently looking at
  (:Pressed
    (Utilities|IsValid (Utilities|ToObject(Interface) _objectlookingat)
      (:Is%20Valid
        (Default|Interact _objectlookingat self)))))

(event Input|AxisEvents|InputAxisMoveForward
  (params (AxisValue :type Float%20%28single-precision%29))
  (Pawn|Input|AddMovementInput (Transformation|GetActorForwardVector) AxisValue false)
  (if (>= (Math|Vector|VectorLength (- (Transformation|GetActorLocation) (Variables|Default|GetLocation))) (Math|Float|MakeLiteralFloat 1e+02))
    (Variables|Default|SetLocation (Transformation|GetActorLocation))
    (CallFunction|Step)))

(event Input|AxisEvents|InputAxisMoveRight
  (params (AxisValue :type Float%20%28single-precision%29))
  (Pawn|Input|AddMovementInput (Transformation|GetActorRightVector) AxisValue false))

(event Input|AxisEvents|InputAxisLookUp
  (params (AxisValue :type Float%20%28single-precision%29))
  (Pawn|Input|AddControllerPitchInput AxisValue))

(event Input|AxisEvents|InputAxisTurn
  (params (AxisValue :type Float%20%28single-precision%29))
  (Pawn|Input|AddControllerYawInput AxisValue))

(fn ConstructionScript)

(fn Conversation)

(fn GameOver
  (CameraFades|StartCameraFade :self (Game|GetPlayerCameraManager 0) :ToAlpha 1.0 :Duration 3.0 :bShouldFadeAudio true :bHoldWhenFinished true))

(fn FilterAnswers
  (params (Dialogue :type Dialogue%20Structure%20Structure))
  (for _array_element (.answers Dialogue)
    (bind _keep (CallFunction|GetFilterCondition (.npcid Dialogue) (.conversationid Dialogue) (.Type (Utilities|Struct|BreakAnswerStructure _array_element))))
    (if _keep
      (Utilities|Array|Add (LocalVariables|GetFilteredAnswersArray) _array_element)))
  (return (LocalVariables|GetFilteredAnswersArray)))

(fn GetFilterCondition
  (params (NpcID :type Integer) (ConversationID :type Integer) (AnswerType :type AnswerType%20Enum :default "NewEnumerator0"))
  (bind _stoneputted (Variables|Default|GetStonePutted))
  (bind _returnvalue (Utilities|Enum|Equal(Enum) AnswerType "NewEnumerator1"))
  (bind _returnvalue_2 (Utilities|Enum|Equal(Enum) AnswerType "NewEnumerator3"))
  (bind _returnvalue_3 (and _returnvalue _stoneputted))
  ;[1 1 1] Switch on NPC
  (switch int NpcID
    (:1
      ;[1 1 1] Satyr NPC asking for a stone
      (if (== ConversationID (Class|KismetSystemLibrary|MakeLiteralInteger 9))
        (bind _exists (Default|FindbyClass (Variables|Default|GetInventoryComponent) "/Game/Blueprints/Objects/MagicStone.MagicStone_C"))
        (if _exists
          (return (or (Utilities|Enum|Equal(Enum) AnswerType "NewEnumerator0") _returnvalue_2))
          (elif _returnvalue_3
            (return _returnvalue_3)
            (else
              (return _returnvalue_2))))))))

(fn GetDefaultSpeed
  (return 4e+02))