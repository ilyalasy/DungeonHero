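; Character inventory that stores items in a dictionary keyed by item type, holding at most one item of each type.
; AddItem ignores types already present, otherwise stores the item and calls its OnAdd with the owning character.
; RemoveItem looks up an item by type, removes it from the dictionary and returns it, without calling anything on the item.
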(fn AddItem
  (params (Item :type Item%20Interface%20Interface))
  (bind _itemsdict (Variables|Default|GetItemsDict))
  (bind _type (Default|GetType Item))
  (if (not (Utilities|Map|Contains _itemsdict _type))
    (Utilities|Map|Add _itemsdict _type Item)
    (Default|OnAdd Item (Variables|Default|GetOwnerCharacter))))

(fn RemoveItem
  (params (ItemType :type ItemType%20Enum :default "NewEnumerator0"))
  (bind _itemsdict (Variables|Default|GetItemsDict))
  (bind (_value _returnvalue) (Utilities|Map|Find _itemsdict ItemType))
  (if _returnvalue
    (bind _output_get (LocalVariables|SetFoundItem _value))
    (Utilities|Map|Remove _itemsdict ItemType)
    (return _output_get)))