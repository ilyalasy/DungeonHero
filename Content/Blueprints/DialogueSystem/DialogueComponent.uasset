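; Dialogue component that serves an NPC's conversation lines and tracks whether it is the first meeting.
; On BeginPlay it restores the first-meet flag from the world save and caches DialogueData table rows matching its NpcID.
; GetLine and HasMoreLines scan those rows by conversation and line ID, using a cursor that resets when the conversation changes.
; A Save event writes the flag back to the save slot, keyed by GetUniqueName.
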(event EventBeginPlay
  (CallFunction|Load)
  (bind _outrownames (DataTable|GetDataTableRowNames "/Game/Blueprints/DialogueSystem/DialogueData.DialogueData"))
  (for _array_element _outrownames
    (bind _returnvalue (Utilities|GetDataTableRow "/Game/Blueprints/DialogueSystem/DialogueData.DialogueData" _array_element)
      (:then
        (if (== (.npcid _returnvalue) (Variables|Default|GetNpcID))
          (Utilities|Array|Add (Variables|Default|GetDialogueRows) _array_element))))))

(event EventSave
  (bind _savegame (CallFunction|GetWorldSave))
  (Utilities|Map|Add (Variables|/Game/Blueprints/Save/WorldSaveGame.WorldSaveGame_C|GetDialogueData _savegame) (Utilities|GetUniqueName) (Utilities|Struct|MakeDialogueSaveData (Variables|Default|GetFirstMeet)))
  (SaveGame|SaveGametoSlot _savegame (Variables|/Game/Blueprints/Save/WorldSaveGame.WorldSaveGame_C|GetSaveGameSlot _savegame) (Variables|/Game/Blueprints/Save/WorldSaveGame.WorldSaveGame_C|GetPlayerID _savegame)))

(event EventLoad
  (bind _savegame (CallFunction|GetWorldSave))
  (if (.ReturnValue (Utilities|Map|Find (Variables|/Game/Blueprints/Save/WorldSaveGame.WorldSaveGame_C|GetDialogueData _savegame) (Utilities|GetUniqueName)))
    (Variables|Default|SetFirstMeet (.firstmeet (.Value (Utilities|Map|Find (Variables|/Game/Blueprints/Save/WorldSaveGame.WorldSaveGame_C|GetDialogueData _savegame) (Utilities|GetUniqueName)))))))

(fn GetLine
  (params (ConversationID :type Integer) (Next :type Boolean))
  (if (== ConversationID (Variables|Default|GetPrevConversationID))
    _
    (else
      (Variables|Default|SetCurrentLineID 1)))
  (for _array_element (Variables|Default|GetDialogueRows)
    (bind _returnvalue (Utilities|GetDataTableRow "/Game/Blueprints/DialogueSystem/DialogueData.DialogueData" _array_element)
      (:then
        (if (and (== ConversationID (.ConversationID (Utilities|Struct|BreakDialogueStructure _returnvalue))) (== (Variables|Default|GetCurrentLineID) (.LineID (Utilities|Struct|BreakDialogueStructure _returnvalue))))
          (if Next
            (Math|Integer|IncrementInt (Variables|Default|GetCurrentLineID)
              (:%20%20
                _)))
          (Variables|Default|SetPrevConversationID ConversationID)
          (return _returnvalue))))))

(fn HasMoreLines
  (params (ConversationID :type Integer))
  (if (== ConversationID (Variables|Default|GetPrevConversationID))
    _
    (else
      (Variables|Default|SetCurrentLineID 1)))
  (for _array_element (Variables|Default|GetDialogueRows)
    (bind _returnvalue (Utilities|GetDataTableRow "/Game/Blueprints/DialogueSystem/DialogueData.DialogueData" _array_element)
      (:then
        (if (and (== (.conversationid _returnvalue) ConversationID) (== (.lineid _returnvalue) (Variables|Default|GetCurrentLineID)))
          (return true)))))
  (return false))

(fn IsFirstMeet
  (if (Variables|Default|GetFirstMeet)
    (Variables|Default|SetFirstMeet false)
    (return true)
    (else
      (return false))))

(fn ToggleTalk
  (Variables|Default|SetIsTalking (not (Variables|Default|GetIsTalking))))