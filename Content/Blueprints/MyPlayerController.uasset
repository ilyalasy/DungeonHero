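; Player controller that applies saved sound and video settings on start and triggers world object saving on shutdown.
; BeginPlay loads the SoundSettingsSave slot, overrides Master, Music and Effects volumes in MasterSoundMix, then applies the game user settings.
; Destroyed and EndPlay both run SaveObjects, which creates a fresh WorldSaveGame and calls Save on every actor implementing the Savable interface.
; SaveObjects itself never writes that save object to a slot.
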(event EventBeginPlay
  ;[1 1 1] Load sound settings
  (CallFunction|LoadSoundSettings)
  ;[1 1 1] Load video settings
  (bind _returnvalue (Settings|GetGameUserSettings))
  (Class|GameUserSettings|ApplySettings _returnvalue false))

(event EventTick
  (params (DeltaSeconds :type Float%20%28single-precision%29)))

(event EventEndPlay
  (params (EndPlayReason :type EEndPlayReason%20Enum :default "Destroyed"))
  (CallFunction|SaveObjects))

(event EventDestroyed
  (CallFunction|SaveObjects))

(fn ConstructionScript)

(fn LoadSoundSettings
  (bind _returnvalue (SaveGame|CreateSaveGameObject "/Game/Blueprints/Save/SoundSettingsSave.SoundSettingsSave_C"))
  (bind _output_get (LocalVariables|SetSoundSettings _returnvalue))
  (bind _returnvalue_2 (SaveGame|DoesSaveGameExist (Variables|/Game/Blueprints/Save/SoundSettingsSave.SoundSettingsSave_C|GetSaveGameSlot _output_get) (Variables|/Game/Blueprints/Save/SoundSettingsSave.SoundSettingsSave_C|GetPlayerID _output_get)))
  (if _returnvalue_2
    (bind _returnvalue_3 (SaveGame|LoadGamefromSlot (Variables|/Game/Blueprints/Save/SoundSettingsSave.SoundSettingsSave_C|GetSaveGameSlot (LocalVariables|GetSoundSettings)) (Variables|/Game/Blueprints/Save/SoundSettingsSave.SoundSettingsSave_C|GetPlayerID (LocalVariables|GetSoundSettings))))
    (bind _assound_settings_save (Utilities|Casting|CastToSoundSettingsSave _returnvalue_3))
    (Audio|SetSoundMixClassOverride "/Game/Audio/MasterSoundMix.MasterSoundMix" "/Game/Audio/Master.Master" (Variables|/Game/Blueprints/Save/SoundSettingsSave.SoundSettingsSave_C|GetMasterVolume _assound_settings_save) 1.0 1.0 true)
    (Audio|SetSoundMixClassOverride "/Game/Audio/MasterSoundMix.MasterSoundMix" "/Game/Audio/Music.Music" (Variables|/Game/Blueprints/Save/SoundSettingsSave.SoundSettingsSave_C|GetMusicVolume _assound_settings_save) 1.0 1.0 true)
    (Audio|SetSoundMixClassOverride "/Game/Audio/MasterSoundMix.MasterSoundMix" "/Game/Audio/Effects.Effects" (Variables|/Game/Blueprints/Save/SoundSettingsSave.SoundSettingsSave_C|GetEffectsVolume _assound_settings_save) 1.0 1.0 true)))

(fn SaveObjects
  (bind _returnvalue (SaveGame|CreateSaveGameObject "/Game/Blueprints/Save/WorldSaveGame.WorldSaveGame_C"))
  (LocalVariables|SetObjectsSave _returnvalue)
  (bind _outactors (Actor|GetAllActorswithInterface "/Game/Blueprints/Save/Savable.Savable_C"))
  (for _array_element _outactors
    (bind _assavable (Utilities|Casting|CastToSavable _array_element))
    (Default|Save _assavable)))