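; Player character with axis-driven movement and look that detects the interactable actor it faces.
; Each Tick, a Visibility line trace runs from the actor's location along its forward vector, not from the camera, and calls OnLookAt on a hit InteractableActor.
; When nothing is hit, it clears the actor name widget through MyHUD and disables input on the last cast InteractableActor, if still valid.
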(event EventTick
  (params (DeltaSeconds :type Float%20%28single-precision%29))
  (bind _returnvalue (Game|GetPlayerController 0))
  (bind _returnvalue_2 (Transformation|GetActorLocation))
  ;[1 1 1] Get object character looking at
  (bind (_outhit _returnvalue_3) (Collision|LineTraceByChannel _returnvalue_2 (+ _returnvalue_2 (* (Transformation|GetActorForwardVector) (Variables|Default|GetTraceDistance))) "TraceTypeQuery1" false 0 "None"))
  (if _returnvalue_3
    (bind _asinteractable_actor (Utilities|Casting|CastToInteractableActor (.HitActor (Collision|BreakHitResult _outhit))))
    (Default|OnLookat _asinteractable_actor)
    (else
      (bind _asmy_hud (Utilities|Casting|CastToMyHUD (HUD|GetHUD _returnvalue)))
      (Default|CallUpdateActorNameWidget _asmy_hud)
      (if (Utilities|IsValid _asinteractable_actor)
        (Input|DisableInput _asinteractable_actor _returnvalue)))))

(event Input|AxisEvents|InputAxisMoveForward
  (params (AxisValue :type Float%20%28single-precision%29))
  (Pawn|Input|AddMovementInput (Transformation|GetActorForwardVector) AxisValue false))

(event Input|AxisEvents|InputAxisMoveRight
  (params (AxisValue :type Float%20%28single-precision%29))
  (Pawn|Input|AddMovementInput (Transformation|GetActorRightVector) AxisValue false))

(event Input|AxisEvents|InputAxisLookUp
  (params (AxisValue :type Float%20%28single-precision%29))
  (Pawn|Input|AddControllerPitchInput AxisValue))

(event Input|AxisEvents|InputAxisTurn
  (params (AxisValue :type Float%20%28single-precision%29))
  (Pawn|Input|AddControllerYawInput AxisValue))

(fn ConstructionScript)