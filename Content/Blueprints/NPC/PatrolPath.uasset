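; Patrol path actor that supplies NPCs with looping path points and target points to move to.
; GetNextPathPoint cycles through local-space PathPoints, converting each to world space through the actor's transform.
; GetNextTargetPoint cycles through TargetPoints, returning each transform with its index and the matching InteractableObjects entry.
; GetRandomTargetPoint returns a random target's transform and sets the current target index from a random pick.
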(event EventBeginPlay)

(event Collision|EventActorBeginOverlap
  (params (OtherActor :type Actor%20Object%20Reference)))

(event EventTick
  (params (DeltaSeconds :type Float%20%28single-precision%29)))

(fn ConstructionScript)

(fn GetNextPathPoint
  (bind _output_get (LocalVariables|SetResult (Math|Transform|TransformLocation (Transformation|GetActorTransform self) (Utilities|Array|Get(acopy) (Variables|Default|GetPathPoints) (Variables|Default|GetCurrentPathIndex)))))
  (Variables|Default|SetCurrentPathIndex (Math|Integer|%(Integer) (+ (Variables|Default|GetCurrentPathIndex) 1) (Utilities|Array|Length (Variables|Default|GetPathPoints))))
  (return _output_get))

(fn GetRandomTargetPoint
  (bind _targetpoints (Variables|Default|GetTargetPoints))
  (bind (_element _index) (Utilities|GetRandomArrayElement _targetpoints))
  (Variables|Default|SetCurrentTargetIndex _index)
  (return (Transformation|GetActorTransform _element)))

(fn GetNextTargetPoint
  (bind _output_get (LocalVariables|SetResult (Transformation|GetActorTransform (Utilities|Array|Get(acopy) (Variables|Default|GetTargetPoints) (Variables|Default|GetCurrentTargetIndex)))))
  (LocalVariables|SetTemp (Variables|Default|GetCurrentTargetIndex))
  (Variables|Default|SetCurrentTargetIndex (Math|Integer|%(Integer) (+ (Variables|Default|GetCurrentTargetIndex) 1) (Utilities|Array|Length (Variables|Default|GetTargetPoints))))
  (return _output_get (LocalVariables|GetTemp) (Utilities|Array|Get(acopy) (Variables|Default|GetInteractableObjects) (LocalVariables|GetTemp))))