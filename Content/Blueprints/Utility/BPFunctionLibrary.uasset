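; Blueprint function library with shared helpers for reaching the world save and the player's HUD.
; GetWorldSave creates a fresh WorldSaveGame to read its slot name and player ID, returning the save loaded from that slot if one exists, otherwise the new unsaved object.
; GetHUD returns the HUD of player controller 0 cast to MyHUD.
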(fn GetWorldSave
  (bind _returnvalue (SaveGame|CreateSaveGameObject "/Game/Blueprints/Save/WorldSaveGame.WorldSaveGame_C"))
  (bind _output_get (LocalVariables|SetWorldSave _returnvalue))
  (bind _returnvalue_2 (SaveGame|DoesSaveGameExist (Variables|/Game/Blueprints/Save/WorldSaveGame.WorldSaveGame_C|GetSaveGameSlot _output_get) (Variables|/Game/Blueprints/Save/WorldSaveGame.WorldSaveGame_C|GetPlayerID _output_get)))
  (if _returnvalue_2
    (bind _returnvalue_3 (SaveGame|LoadGamefromSlot (Variables|/Game/Blueprints/Save/WorldSaveGame.WorldSaveGame_C|GetSaveGameSlot (LocalVariables|GetWorldSave)) (Variables|/Game/Blueprints/Save/WorldSaveGame.WorldSaveGame_C|GetPlayerID (LocalVariables|GetWorldSave))))
    (bind _asworld_save_game (Utilities|Casting|CastToWorldSaveGame _returnvalue_3))
    (LocalVariables|SetWorldSave _asworld_save_game))
  (return (LocalVariables|GetWorldSave)))

(fn GetHUD
  (bind _asmy_hud (Utilities|Casting|CastToMyHUD (HUD|GetHUD (Game|GetPlayerController (LocalVariables|Get__WorldContext)))))
  (return _asmy_hud))